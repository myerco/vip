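; First-person hero character that handles player look, movement, jumping, sprinting and shooting.
; On BeginPlay it sets walking speed, then spawns a BP_SKFGun and attaches it to the right-hand socket of the Bracos arms.
; Sprint input switches max walk speed between walking and running values, while fire input forwards trigger press and release to the gun.
; Both inputs also maintain EstaCorrendo and EstaAtirando state flags.
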(event EventBeginPlay
  (bind _bracos (Variables|Default|GetBracos))
  (Utilities|FlowControl|Sequence
    (:then_0
      ;[1 1 1] Incializa Velocidade
      (Variables|/Script/Engine.CharacterMovementComponent|SetMaxWalkSpeed (Variables|Character|GetCharacterMovement) (Variables|Default|GetVelocidadeAndando)))
    (:then_1
      ;[1 1 1] Inicializa Arma
      (bind _returnvalue (Game|SpawnActorfromClass "/Game/Blueprints/Armas/SKF_Gun/BP_SKFGun.BP_SKFGun_C" (Transformation|GetWorldTransform _bracos) "Undefined" 0 0))
      (bind _output_get (Variables|Default|SetRefArma _returnvalue))
      (Transformation|AttachComponentToComponent _output_get _bracos "hand_rSocket" "SnapToTarget" "SnapToTarget" "SnapToTarget" true))))

(event Input|ActionEvents|InputActionBotaoAtirar
  (params (Key :type Key%20Structure))
  (bind _refarma (Variables|Default|GetRefArma))
  ;[1 1 1] Atirando
  (:Pressed
    (Default|AcionaGatilho _refarma)
    (Variables|Default|SetEstaAtirando true))
  (:Released
    (Default|DesabilitaGatilho _refarma)
    (Variables|Default|SetEstaAtirando false)))

(event Input|ActionEvents|InputActionBotaoCorrer
  (params (Key :type Key%20Structure))
  (bind _charactermovement (Variables|Character|GetCharacterMovement))
  ;[1 1 1] Correndo
  (:Pressed
    (Variables|Default|SetEstaCorrendo true)
    (Variables|/Script/Engine.CharacterMovementComponent|SetMaxWalkSpeed _charactermovement (Variables|Default|GetVelocidadeCorrendo)))
  (:Released
    (Variables|Default|SetEstaCorrendo false)
    (Variables|/Script/Engine.CharacterMovementComponent|SetMaxWalkSpeed _charactermovement (Variables|Default|GetVelocidadeAndando))))

(event Input|ActionEvents|InputActionBotaoPular
  (params (Key :type Key%20Structure))
  ;[1 1 1] Pula
  (:Pressed
    (Character|Jump))
  (:Released
    (Character|StopJumping)))

(event Input|AxisEvents|InputAxisMouseCima
  (params (AxisValue :type Float%20%28single-precision%29))
  ;[1 1 1] Mouse
  (Pawn|Input|AddControllerPitchInput AxisValue))

(event Input|AxisEvents|InputAxisMouseVira
  (params (AxisValue :type Float%20%28single-precision%29))
  ;[1 1 1] Mouse
  (Pawn|Input|AddControllerYawInput AxisValue))

(event Input|AxisEvents|InputAxisTecladoFrente
  (params (AxisValue :type Float%20%28single-precision%29))
  ;[1 1 1] Teclado movimento
  (Pawn|Input|AddMovementInput (Math|Vector|GetForwardVector (Variables|Collision|GetCapsuleComponent)) AxisValue false))

(event Input|AxisEvents|InputAxisTecladoDireita
  (params (AxisValue :type Float%20%28single-precision%29))
  ;[1 1 1] Teclado movimento
  (Pawn|Input|AddMovementInput (Math|Vector|GetRightVector (Variables|Collision|GetCapsuleComponent)) AxisValue false))

(fn ConstructionScript)