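; BP_Inimigo is an enemy actor that turns to face the player character and is destroyed when its health runs out.
; Overlap with Colisao toggles a sighting flag, while being hit sets a permanent alert flag; either makes Tick rotate it toward the player.
; Each hit subtracts Dano from Vida, without checking what struck it.
; The Movimento timeline defines a randomised vertical lerp from the spawn point, but no graph event starts it.
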(event OnComponentBeginOverlap(Colisao)
  (params (OverlappedComponent :type Primitive%20Component%20Object%20Reference) (OtherActor :type Actor%20Object%20Reference) (OtherComp :type Primitive%20Component%20Object%20Reference) (OtherBodyIndex :type Integer) (bFromSweep :type Boolean) (SweepResult :type Hit%20Result%20Structure%20%28by%20ref%29))
  ;[1 1 1] Personagem a vista
  (Variables|Default|SetEstaAVista true))

(event OnComponentEndOverlap(Colisao)
  (params (OverlappedComponent :type Primitive%20Component%20Object%20Reference) (OtherActor :type Actor%20Object%20Reference) (OtherComp :type Primitive%20Component%20Object%20Reference) (OtherBodyIndex :type Integer))
  ;[1 1 1] Personagem sai de vista
  (Variables|Default|SetEstaAVista false))

(event EventBeginPlay
  (bind _returnvalue (Transformation|GetActorLocation))
  (Utilities|FlowControl|Sequence
    (:then_0
      ;[1 1 1] Inicializa Movimento
      (Variables|Default|SetPosInicial _returnvalue)
      (Variables|Default|SetPosFinal (+ _returnvalue (Math|Vector|MakeVector 0.0 0.0 (Math|Random|RandomFloatinRange 5e+01 1e+02))))
      (Components|Timeline|SetPlayRate (Variables|Default|GetMovimento) (Math|Random|RandomFloatinRange 1.0 2.0)))
    (:then_1
      ;[1 1 1] Inicializa personagem
      (bind _asbp_personagem_hero (Utilities|Casting|CastToBP_PersonagemHero (Game|GetPlayerCharacter 0)))
      (Variables|Default|SetRefPersonagem _asbp_personagem_hero))))

(event Collision|EventHit
  (params (MyComp :type Primitive%20Component%20Object%20Reference) (Other :type Actor%20Object%20Reference) (OtherComp :type Primitive%20Component%20Object%20Reference) (bSelfMoved :type Boolean) (HitLocation :type Vector :default "0, 0, 0") (HitNormal :type Vector :default "0, 0, 0") (NormalImpulse :type Vector :default "0, 0, 0") (Hit :type Hit%20Result%20Structure%20%28by%20ref%29))
  ;[1 1 1] Atingido pelo projetil
  (Variables|Default|SetEstaAqui true)
  (bind _output_get (Variables|Default|SetVida (- (Variables|Default|GetVida) (Variables|Default|GetDano))))
  (if (<= _output_get 0.0)
    (Development|PrintString "Morreu")
    (Actor|DestroyActor)))

(event EventTick
  (params (DeltaSeconds :type Float%20%28single-precision%29))
  ;[1 1 1] Animação de inimigo
  (if (or (Variables|Default|GetEstaAVista) (Variables|Default|GetEstaAqui))
    (Transformation|SetActorRotation (Math|Rotator|FindLookatRotation (Transformation|GetActorLocation) (Transformation|GetActorLocation (Variables|Default|GetRefPersonagem))))))

(fn ConstructionScript)