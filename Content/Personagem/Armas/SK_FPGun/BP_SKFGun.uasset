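; BP_SKFGun is a weapon Blueprint for the player hero that fires projectiles automatically while its trigger is engaged.
; BeginPlay caches the player character as BP_PersonagemHero.
; AcionaGatilho fires at once and starts a looping timer on Dispara at the TirosPorSegundo rate; DesabilitaGatilho clears it.
; Each shot spawns a BP_Projetil at the location and rotation of the hero's DirecaoProjetil component, rather than from the gun itself.
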(event Custom|AcionaGatilho
  ;[1 1 1] Aciona e Desabilita Gatilho
  (CallFunction|Dispara)
  (Utilities|Time|SetTimerbyFunctionName 0 "Dispara" (/ 1.0 (Variables|Default|GetTirosPorSegundo)) true))

(event Custom|DesabilitaGatilho
  ;[1 1 1] Aciona e Desabilita Gatilho
  (Utilities|Time|ClearTimerbyFunctionName 0 "Dispara"))

(event EventBeginPlay
  ;[1 1 1] Inicializa o personagem
  (bind _asbp_personagem_hero (Utilities|Casting|CastToBP_PersonagemHero (Game|GetPlayerCharacter 0)))
  (Variables|Default|SetRefPersonagemHero _asbp_personagem_hero))

(fn ConstructionScript)

(fn Dispara
  (bind _refpersonagemhero (Variables|Default|GetRefPersonagemHero))
  (bind _direcaoprojetil (Variables|/Game/Personagem/BP_PersonagemHero.BP_PersonagemHero_C|GetDirecaoProjetil _refpersonagemhero))
  (bind _returnvalue (Transformation|GetWorldTransform _direcaoprojetil))
  (Game|SpawnActorfromClass "/Game/Personagem/Armas/BP_Projetil.BP_Projetil_C" (Math|Transform|MakeTransform (.location _returnvalue) (.rotation _returnvalue) "1,1,1") "Undefined" 0 0))